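; BP_PlayerCharacter is a player character that handles basic looking, jumping and movement from Enhanced Input actions.
; Look input feeds controller yaw and pitch, and the jump action starts and stops the built-in character jump.
; Movement input follows control rotation with pitch zeroed, so forward movement uses only yaw while strafing uses yaw and roll.
; BeginPlay and the construction script are empty.
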(event Input|EnhancedActionEvents|EnhancedInputActionInput_Jump
  (params (ActionValue :type Boolean) (ElapsedSeconds :type Float%20%28double-precision%29) (TriggeredSeconds :type Float%20%28double-precision%29) (InputAction :type Input%20Action%20Object%20Reference :default "/Game/Input/Input_Jump.Input_Jump"))
  (:Triggered
    (Character|Jump))
  (:Canceled
    (Character|StopJumping)))

(event Input|EnhancedActionEvents|EnhancedInputActionInput_Movement
  (params (ActionValue :type Vector%202D%20Structure) (ElapsedSeconds :type Float%20%28double-precision%29) (TriggeredSeconds :type Float%20%28double-precision%29) (InputAction :type Input%20Action%20Object%20Reference :default "/Game/Input/Input_Movement.Input_Movement"))
  (bind _returnvalue (Pawn|GetControlRotation :!class /Script/Engine.Pawn))
  (Pawn|Input|AddMovementInput (Math|Vector|GetRightVector (Math|Rotator|MakeRotator (.roll _returnvalue) 0.0 (.yaw _returnvalue))) (.x ActionValue) false)
  (Pawn|Input|AddMovementInput (Math|Vector|GetForwardVector (Math|Rotator|MakeRotator 0.0 0.0 (.yaw _returnvalue))) (.y ActionValue) false))

(event Input|EnhancedActionEvents|EnhancedInputActionInput_Look
  (params (ActionValue :type Vector%202D%20Structure) (ElapsedSeconds :type Float%20%28double-precision%29) (TriggeredSeconds :type Float%20%28double-precision%29) (InputAction :type Input%20Action%20Object%20Reference :default "/Game/Input/Input_Look.Input_Look"))
  (Pawn|Input|AddControllerYawInput (.x ActionValue))
  (Pawn|Input|AddControllerPitchInput (.y ActionValue)))

(event EventBeginPlay)

(fn ConstructionScript)